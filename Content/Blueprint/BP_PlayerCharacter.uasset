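; Player character Blueprint that equips two guns and switches between them with the 1 and 2 keys.
; On BeginPlay it assigns mesh and camera references, then attaches the Vector and ShotGun child-actor components to the arm's GripPoint socket.
; Both child actors are cast to Gun and stored in an array, with SetGunIndex selecting the active one.
; BeginPlay also adds the PlayerUI widget to the viewport and selects the first gun.
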(event Collision|EventActorBeginOverlap
  (params (OtherActor :type Actor%20Object%20Reference)))

(event EventBeginPlay
  (bind _bp_shotgun (Variables|Default|GetBP_ShotGun))
  (Variables|Default|SetArmMesh (Variables|Default|Getarm))
  (Variables|Default|SetGunMesh (Variables|Default|GetBaseGun))
  (Variables|Default|SetCameraComponent (Variables|Default|GetCamera))
  (Transformation|AttachComponentToComponent (Variables|Default|GetBP_Vector) (Variables|Default|Getarm) "GripPoint" "KeepWorld" "KeepWorld" "KeepWorld" true)
  (bind _asgun (Utilities|Casting|CastToGun (Variables|/Script/Engine.ChildActorComponent|GetChildActor (Variables|Default|GetBP_Vector))))
  (Utilities|Array|Add (Variables|Default|Getgun) _asgun)
  (Transformation|AttachComponentToComponent _bp_shotgun (Variables|Default|Getarm) "GripPoint" "KeepRelative" "SnapToTarget" "KeepRelative" true)
  (Transformation|AddLocalRotation _bp_shotgun "0.000000,90.000000, 0" false false)
  (bind _asgun_2 (Utilities|Casting|CastToGun (Variables|/Script/Engine.ChildActorComponent|GetChildActor (Variables|Default|GetBP_ShotGun))))
  (Utilities|Array|Add (Variables|Default|Getgun) _asgun_2)
  (bind _returnvalue (UserInterface|CreateWidget "/Game/Resource/Widget/PlayerUI.PlayerUI_C"))
  (UserInterface|Viewport|AddtoViewport _returnvalue 0)
  (Class|PlayerCharacter|SetGunIndex))

(event Input|KeyboardEvents|1
  (params (Key :type Key%20Structure :default "None"))
  (:Pressed
    (Class|PlayerCharacter|SetGunIndex)))

(event Input|KeyboardEvents|2
  (params (Key :type Key%20Structure :default "None"))
  (:Pressed
    (Class|PlayerCharacter|SetGunIndex 1)))

(fn ConstructionScript)